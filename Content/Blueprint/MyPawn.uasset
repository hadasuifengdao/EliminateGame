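; MyPawn is a pawn Blueprint that handles the Rechoose menu and passes score to the game instance.
; The ReChoose input toggles a Rechoose widget on and off, tracked by MenuOn.
; Every Tick it finds all BlockGrid actors and copies their Score into the custom Instance game instance.
; A custom start event plays a timeline in reverse from its end, writing the track value to Time.
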(event Custom|start
  (bind _newtrack_0 (Timeline|Timeline_0 ReverseFromEnd)
    (:Update
      (Variables|Default|Settime _newtrack_0))))

(event EventBeginPlay)

(event Collision|EventActorBeginOverlap
  (params (OtherActor :type Actor%20Object%20Reference)))

(event EventTick
  (params (DeltaSeconds :type Float%20%28single-precision%29))
  (bind _outactors (Actor|GetAllActorsOfClass "/Script/xiaoxiaole.BlockGrid"))
  (for _array_element _outactors
    (bind _asinstance (Utilities|Casting|CastToInstance (Game|GetGameInstance)))
    (Variables|/Game/UMG/Instance.Instance_C|SetScore _asinstance (Variables|/Script/xiaoxiaole.BlockGrid|GetScore _array_element))))

(event Input|ActionEvents|InputActionReChoose
  (params (Key :type Key%20Structure :default "AnyKey"))
  (:Pressed
    (if (Variables|Default|GetMenuOn)
      (Widget|RemovefromParent (stale _returnvalue))
      (Variables|Default|SetMenuOn false)
      (else
        (bind _returnvalue (UserInterface|CreateWidget "/Game/UMG/Rechoose.Rechoose_C"))
        (UserInterface|Viewport|AddtoViewport _returnvalue 0)
        (Variables|Default|SetMenuOn true)))))

(fn ConstructionScript)